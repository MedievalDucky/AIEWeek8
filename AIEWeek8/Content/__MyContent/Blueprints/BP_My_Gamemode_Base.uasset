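; Base game mode Blueprint that links to the level's game manager and provides the setup for the game's UI.
; BeginPlay caches the first BP_My_gamemanager actor found in the world.
; CreateUI, not called within this graph, builds the Abandon, Win, Lose and Health widgets, stores each on the game manager and adds all of them to the viewport immediately.
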(event `self.ReceiveBeginPlay`
  (bind _outactors (`GameplayStatics.GetAllActorsOfClass` "/Game/__MyContent/Blueprints/BP_My_gamemanager.BP_My_gamemanager_C"))
  (set `self.My Game manager` (`|GetArrayItem` _outactors)))

(fn `Create UI`
  (bind _my_game_manager1 (`/Game/__MyContent/Blueprints/BP_My_Funciton_Library.Get my game manager` null))
  (bind _returnvalue (`|CreateWidget` "/Game/__MyContent/UI/Widget_Abandon.Widget_Abandon_C"))
  (bind _output_get (set `/Game/__MyContent/Blueprints/BP_My_gamemanager.Widget_abandon` _returnvalue _my_game_manager1))
  (`UserWidget.AddToViewport` _output_get 0)
  (bind _returnvalue_2 (`|CreateWidget` "/Game/__MyContent/UI/Widget_Win.Widget_Win_C"))
  (bind _output_get_2 (set `/Game/__MyContent/Blueprints/BP_My_gamemanager.widget win` _returnvalue_2 _my_game_manager1))
  (`UserWidget.AddToViewport` _output_get_2 0)
  (bind _returnvalue_3 (`|CreateWidget` "/Game/__MyContent/UI/Widget_Lose.Widget_Lose_C"))
  (bind _output_get_3 (set `/Game/__MyContent/Blueprints/BP_My_gamemanager.widget lose` _returnvalue_3 _my_game_manager1))
  (`UserWidget.AddToViewport` _output_get_3 0)
  (bind _returnvalue_4 (`|CreateWidget` "/Game/__MyContent/UI/Widget_Health.Widget_Health_C"))
  (bind _output_get_4 (set `/Game/__MyContent/Blueprints/BP_My_gamemanager.Widget Health` _returnvalue_4 _my_game_manager1))
  (`UserWidget.AddToViewport` _output_get_4 0))

(fn `UserConstructionScript`)